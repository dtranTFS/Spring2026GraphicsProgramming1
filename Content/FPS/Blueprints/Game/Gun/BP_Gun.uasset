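; BP_Gun is a gun Blueprint that exposes damage, fire rate and shoot distance through getter functions.
; Its interface shoot event forwards the start and end positions to OnBlueprintShoot.
; OnBlueprintShoot is a placeholder that only prints a debug string, with no trace or damage logic.
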(event `/Game/FPS/Blueprints/Game/Gun/BPI_Gun.OnInterfaceShoot`
  (params (StartPos :type "Vector Structure") (EndPos :type "Vector Structure"))
  (`self.OnBlueprintShoot` StartPos EndPos))

(fn `GetDamage`
  (returns (Damage :type "Float (double-precision)"))
  (return (`self.Damage`)))

(fn `GetFireRate`
  (returns (FireRate :type "Float (double-precision)"))
  (return (`self.FireRate`)))

(fn `GetShootDistance`
  (returns (ShootDistance :type "Float (double-precision)"))
  (return (`self.ShootDistance`)))

(fn `OnBlueprintShoot`
  (params (StartPos :type "Vector Structure") (EndPos :type "Vector Structure"))
  (`KismetSystemLibrary.PrintString` "Gun Shoot Called"))

(fn `UserConstructionScript`)