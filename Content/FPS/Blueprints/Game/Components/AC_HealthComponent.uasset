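; Actor component for the FPS game that stores an actor's health and exposes damage, heal, full heal, kill, percentage and death queries.
; All changes go through SetHealth, which clamps to the min/max range; Damage and Heal print an error for non-positive amounts.
; Init sets health before assigning the new bounds, so the starting value is clamped against the previous range.
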(fn `ClampHealth`
  (params (Value :type "Float (double-precision)"))
  (returns (ReturnValue :type "Float (double-precision)"))
  (return (`KismetMathLibrary.FClamp` Value (`self.MinHealth`) (`self.MaxHealth`))))

(fn `Damage`
  (params (Amount :type "Float (double-precision)"))
  (if (> Amount 0.0)
    (`self.SetHealth` (- (`self.GetHealth`) Amount))
    (else
      (`KismetSystemLibrary.PrintString` "Damage value must be positive! Stupid"))))

(fn `GetHealth`
  (returns (Health :type "Float (double-precision)"))
  (return (`self.Health`)))

(fn `GetPercentHealth`
  (returns (Percent :type "Float (double-precision)"))
  (return (`KismetMathLibrary.FClamp` (/ (`self.GetHealth`) (`self.MaxHealth`)))))

(fn `Heal`
  (params (Amount :type "Float (double-precision)"))
  (if (> Amount 0.0)
    (`self.SetHealth` (+ (`self.GetHealth`) Amount))
    (else
      (`KismetSystemLibrary.PrintString` "Heal value must be positive! Stupid"))))

(fn `HealFull`
  (`self.Heal` (`self.MaxHealth`)))

(fn `Init`
  (params (Health :type "Float (double-precision)") (MinHealth :type "Float (double-precision)") (MaxHealth :type "Float (double-precision)"))
  (`self.SetHealth` Health)
  (set `self.MinHealth` MinHealth)
  (set `self.MaxHealth` MaxHealth))

(fn `IsDead`
  (returns (IsDead :type Boolean))
  (return (<= (`self.GetHealth`) (`self.MinHealth`))))

(fn `Kill`
  (`self.Damage` (`self.MaxHealth`)))

(fn `SetHealth`
  (params (NewHealth :type "Float (double-precision)"))
  (returns (Health :type "Float (double-precision)"))
  (bind _output_get (set `self.Health` (`self.ClampHealth` NewHealth)))
  (return _output_get))