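; First-person shooter player that moves, looks, jumps and fires a gun spawned at BeginPlay, using Enhanced Input.
; Shots go through gun interface messages along a camera-forward line, after a fire-rate delay.
; A health component feeds the GameManager's health bar, and its game-over event kills the player and loads the main menu.
; Jumping adds score and each shot also damages the player, which looks like test wiring.
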(event `self.ReceiveBeginPlay`
  (`KismetSystemLibrary.PrintString` "Player Spawning" true true (struct :`G` 1.0 :`A` 1.0) 5.0)
  (`self.SetupEnhancedInput`)
  (`self.SpawnGun` (`self.StartingGun`))
  (`/Game/FPS/Blueprints/Game/Components/AC_HealthComponent.Init` (`self.AC_HealthComponent`) 100.0 0.0 100.0)
  (`self.UpdateHealthBarUI`)
  (bind _asbp_game_manager (cast `/Game/FPS/Blueprints/Game/BP_GameManager` (`GameplayStatics.GetGameMode`)))
  (add `/Game/FPS/Blueprints/Game/BP_GameManager.GameOver` _asbp_game_manager (delegate `GameOver`)))

(event `GameOver`
  (`/Game/FPS/Blueprints/Game/Components/AC_HealthComponent.Kill` (`self.AC_HealthComponent`))
  (`self.DisableInput` (`GameplayStatics.GetPlayerController` 0))
  (`KismetSystemLibrary.Delay` 2.0)
  (`GameplayStatics.OpenLevelBySoftObjectPtr` "/Game/FPS/Maps/MainMenuMap.MainMenuMap"))

(event `EnhancedInput|/Game/FPS/Input/IA_Move`
  (params (ActionValue :type "Vector2D Structure") (ElapsedSeconds :type "Float (double-precision)") (TriggeredSeconds :type "Float (double-precision)") (InputAction :type "InputAction Object Reference" :default "/Game/FPS/Input/IA_Move.IA_Move"))
  ; Movement
  (:`Triggered`
    (`self.AddMovementInput` (`self.GetActorForwardVector`) ActionValue_Y)
    (`self.AddMovementInput` (`self.GetActorRightVector`) ActionValue_X)))

(event `EnhancedInput|/Game/FPS/Input/IA_Jump`
  (params (ActionValue :type Boolean) (ElapsedSeconds :type "Float (double-precision)") (TriggeredSeconds :type "Float (double-precision)") (InputAction :type "InputAction Object Reference" :default "/Game/FPS/Input/IA_Jump.IA_Jump"))
  ; Jumping
  (:`Triggered`
    (`self.Jump`))
  (:`Started`
    (bind _returnvalue (`GameplayStatics.GetActorOfClass` "/Game/FPS/Blueprints/Game/BP_ScoreManager.BP_ScoreManager_C"))
    (`/Game/FPS/Blueprints/Game/BP_ScoreManager.AddToScore` _returnvalue 1)))

(event `EnhancedInput|/Game/FPS/Input/IA_Look`
  (params (ActionValue :type "Vector2D Structure") (ElapsedSeconds :type "Float (double-precision)") (TriggeredSeconds :type "Float (double-precision)") (InputAction :type "InputAction Object Reference" :default "/Game/FPS/Input/IA_Look.IA_Look"))
  ; Looking Around
  (:`Triggered`
    (`self.AddControllerYawInput` ActionValue_X)
    (`self.AddControllerPitchInput` ActionValue_Y)))

(event `EnhancedInput|/Game/FPS/Input/IA_Fire`
  (params (ActionValue :type Boolean) (ElapsedSeconds :type "Float (double-precision)") (TriggeredSeconds :type "Float (double-precision)") (InputAction :type "InputAction Object Reference" :default "/Game/FPS/Input/IA_Fire.IA_Fire"))
  (bind (_startpos _endpos) (`self.CalculateShootStartEnd`))
  (:`Triggered`
    (bind _firerate (message `/Game/FPS/Blueprints/Game/Gun/BPI_Gun.GetFireRate` (`self.GunRef`)))
    (`KismetSystemLibrary.Delay` _firerate)
    (message `/Game/FPS/Blueprints/Game/Gun/BPI_Gun.OnInterfaceShoot` (`self.GunRef`) _startpos _endpos)
    (`self.OnDamagePlayer` 10.0)))

(fn `CalculateShootStartEnd`
  (returns (StartPos :type "Vector Structure") (EndPos :type "Vector Structure"))
  (bind _camera (`self.Camera`))
  (bind _returnvalue (`SceneComponent.K2_GetComponentLocation` _camera))
  (bind _shootdistance (message `/Game/FPS/Blueprints/Game/Gun/BPI_Gun.GetShootDistance` (`self.GunRef`)))
  (return _returnvalue (+ _returnvalue (* (`SceneComponent.GetForwardVector` _camera) _shootdistance))))

(fn `OnDamagePlayer`
  (params (Amount :type "Float (double-precision)"))
  (`/Game/FPS/Blueprints/Game/Components/AC_HealthComponent.Damage` (`self.AC_HealthComponent`) Amount)
  (`self.UpdateHealthBarUI`))

(fn `OnHealPlayer`
  (params (Amount :type "Float (double-precision)"))
  (`/Game/FPS/Blueprints/Game/Components/AC_HealthComponent.Heal` (`self.AC_HealthComponent`) Amount)
  (`self.UpdateHealthBarUI`))

(fn `SetupEnhancedInput`
  (bind _asplayer_controller (cast `PlayerController` (`self.GetController`)))
  (bind _returnvalue (pcsubsystem `EnhancedInputLocalPlayerSubsystem` _asplayer_controller))
  (`/Engine/EditorBlueprintResources/StandardMacros.IsValid` _returnvalue
    (:`Is Valid`
      (`EnhancedInputSubsystemInterface.AddMappingContext` _returnvalue "/Game/FPS/Input/IMC_Player.IMC_Player" 0 (struct)))))

(fn `SpawnGun`
  (params (GunToSpawn :type "Actor Class Reference"))
  (bind _returnvalue (`|SpawnActorFromClass` GunToSpawn (`KismetMathLibrary.MakeTransform` (0.0 0.0 0.0)) "Undefined" "MultiplyWithRoot" null null))
  (bind _output_get (set `self.GunRef` _returnvalue))
  (`self.K2_AttachToComponent` _output_get (`self.GunSpawnPoint`) "None" "SnapToTarget" "SnapToTarget" "SnapToTarget" true))

(fn `UpdateHealthBarUI`
  (bind _asbp_game_manager (cast `/Game/FPS/Blueprints/Game/BP_GameManager` (`GameplayStatics.GetGameMode`)))
  (`/Game/FPS/Blueprints/Game/GUI/WBP_GameMenu.UpdateHealthBar` (`/Game/FPS/Blueprints/Game/BP_GameManager.GameMenu` _asbp_game_manager) (`/Game/FPS/Blueprints/Game/Components/AC_HealthComponent.GetPercentHealth` (`self.AC_HealthComponent`))))

(fn `UserConstructionScript`)