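; AI controller for enemies that runs the BT_EnemyAI behavior tree on BeginPlay and tracks whether it can see the player.
; When PawnSensing spots a BP_Player, it writes a can-see flag and the player object to the Blackboard.
; A retriggerable delay of twice the sensing interval resets the flag and player object once sightings stop, since PawnSensing has no lost-sight event here.
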(event `self.ReceiveBeginPlay`
  (`self.RunBehaviorTree` "/Game/FPS/Blueprints/Game/Enemy/EnemyAI/BT_EnemyAI.BT_EnemyAI"))

(event `self.PawnSensing.OnSeePawn`
  (params (Pawn :type "Pawn Object Reference"))
  (bind _asbp_player (cast `/Game/FPS/Blueprints/Game/BP_Player` Pawn))
  (`self.SetBlackboardCanSeePlayer` true _asbp_player)
  (`KismetSystemLibrary.RetriggerableDelay` (* (`PawnSensingComponent.SensingInterval` (`self.PawnSensing`)) 2.0))
  (`self.SetBlackboardCanSeePlayer` false))

(fn `SetBlackboardCanSeePlayer`
  (params (CanSeePlayer :type Boolean) (PlayerObject :type "Object Object Reference"))
  (locals (BBCabSeePlayer :type Name :default "CanSeePlayer") (BBPlayerObject :type Name :default "Player"))
  (bind _blackboard (`self.Blackboard`))
  (`BlackboardComponent.SetValueAsBool` _blackboard (`local.BBCabSeePlayer`) CanSeePlayer)
  (`BlackboardComponent.SetValueAsObject` _blackboard (`local.BBPlayerObject`) PlayerObject))

(fn `UserConstructionScript`)