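; BP_EnemyThatsGun is an FPS enemy Blueprint that, going by its name, acts as a gun.
; It overrides getters to supply fixed damage, fire rate and an effectively unlimited shoot distance.
; Its shoot interface event only prints a debug message, with no firing logic in this Blueprint.
; OnDamage calls the parent implementation, then destroys the actor on any hit regardless of the damage amount.
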(event `/Game/FPS/Blueprints/Game/Gun/BPI_Gun.OnInterfaceShoot`
  (params (StartPos :type "Vector Structure") (EndPos :type "Vector Structure"))
  (`KismetSystemLibrary.PrintString` "Enemy is shooting"))

(fn `GetDamage`
  (returns (Damage :type "Float (double-precision)"))
  (return 100.0))

(fn `GetFireRate`
  (returns (FireRate :type "Float (double-precision)"))
  (return 1.0))

(fn `GetShootDistance`
  (returns (ShootDistance :type "Float (double-precision)"))
  (return 1000000000.0))

(fn `OnDamage`
  (params (Damage :type "Float (double-precision)"))
  (`parent.OnDamage` Damage)
  (`self.K2_DestroyActor`))

(fn `UserConstructionScript`
  (`parent.UserConstructionScript`))